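; BP_CrowdController is an AI controller for BP_PLEAgent crowd pawns.
; On possess, it casts the pawn to BP_PLEAgent and caches the reference, which is its only active logic.
; Disconnected graphs hold unused logic for wandering to random navigable points and writing the agent's GoalActor to the TargetActor Blackboard key.
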(event EventBeginPlay)

(event EventTick
  (params (DeltaSeconds :type Float%20%28single-precision%29)))

(event EventPossess
  (params (PossessedPawn :type Pawn%20Object%20Reference))
  (bind _asbp_pleagent (Utilities|Casting|CastToBP_PLEAgent PossessedPawn))
  (bind _output_get (Variables|Default|SetAs%20BP%20PLEAgent _asbp_pleagent)))

(fn ConstructionScript)